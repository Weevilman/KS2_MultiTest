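; Base-style grabbable physics actor that motion controllers pick up and drop, located in the Bowling content.
; Pickup branches on GrabType: snap attachment, a runtime-created physics handle, or a runtime physics constraint that auto-releases after a short delay.
; While a handle is held, a tick gate moves its target to the grabbing component, with an optional GrabOffset shaping the grip.
; ForceDrop makes the holding BP_MotionController release it for hand-to-hand grabs.
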(event Custom|Tick%20Handle
  (bind _parent_comp (Variables|Default|GetParent%20Comp))
  (bind _physhandle (Variables|Default|GetPhysHandle))
  (bind _returnvalue (Transformation|GetWorldTransform _parent_comp))
  ;[1 1 1] Update Physics handle
  (Utilities|FlowControl|Gate true
    (:Exit
      (Physics|Components|PhysicsHandle|SetTargetLocation _physhandle (.location _returnvalue))
      (Class|PhysicsHandleComponent|SetTargetRotation _physhandle (.rotation _returnvalue)))))

(event Custom|Constraint%20Grab
  (params (New%20Parent :type Scene%20Component%20Object%20Reference))
  (bind _output_get (Variables|Default|SetParent%20Comp New%20Parent))
  (bind _asprimitive_component (Utilities|Casting|CastToPrimitiveComponent _output_get))
  (bind _returnvalue (AddComponent|AddPhysicsConstraintComponent false))
  (Variables|Default|SetGrab%20Constraint _returnvalue)
  (Class|PhysicsConstraintComponent|SetConstrainedComponents _returnvalue _asprimitive_component "None" (Variables|Default|GetMesh) "None")
  (Utilities|FlowControl|Delay 1.6)
  (Class|PhysicsConstraintComponent|SetConstrainedComponents (Variables|Default|GetGrab%20Constraint) 0 "None" 0 "None")
  (Components|DestroyComponent (Variables|Default|GetGrab%20Constraint)))

(event Custom|Start%20Handle%20Update
  (bind _parent_comp (Variables|Default|GetParent%20Comp))
  (bind _physhandle (Variables|Default|GetPhysHandle))
  (bind _returnvalue (Transformation|GetWorldTransform _parent_comp))
  ;[1 1 1] Update Physics handle
  (Utilities|FlowControl|Gate true) ; enters at Open
)

(event Custom|Release%20Handle
  (bind _physhandle (Variables|Default|GetPhysHandle))
  (bind _physhandle_2 (Variables|Default|GetPhysHandle))
  ;[1 1 1] Update Physics handle
  (Physics|Components|PhysicsHandle|ReleaseComponent _physhandle)
  (Variables|Default|SetParent%20Comp 0)
  (Components|DestroyComponent _physhandle)
  (Utilities|FlowControl|Gate true) ; enters at Close
)

(event Custom|Constraint%20Release
  (bind _grab_constraint (Variables|Default|GetGrab%20Constraint))
  (Class|PhysicsConstraintComponent|SetConstrainedComponents _grab_constraint 0 "None" 0 "None")
  (Components|DestroyComponent _grab_constraint))

(event Custom|Physics%20Handle%20Grab
  (params (Parent :type Scene%20Component%20Object%20Reference) (DistanceGrab :type Boolean))
  (bind _mesh (Variables|Default|GetMesh))
  (bind _graboffset (Variables|Default|GetGrabOffset))
  (bind _returnvalue (Transformation|GetWorldLocation _graboffset))
  (bind _returnvalue_2 (Transformation|GetWorldRotation _graboffset))
  (bind _output_get (Variables|Default|SetParent%20Comp Parent))
  ;[1 1 1] Physics Handle Grab
  (bind _returnvalue_3 (AddComponent|AddPhysicsHandleComponent))
  (bind _output_get_2 (Variables|Default|SetPhysHandle _returnvalue_3))
  (if (Variables|Default|GetUse%20Grab%20Offset)
    (Class|PhysicsHandleComponent|SetTargetLocationandRotation _output_get_2 _returnvalue _returnvalue_2)
    (else
      (Class|PhysicsHandleComponent|SetTargetLocationandRotation _output_get_2 (.location (Transformation|GetWorldTransform _output_get)) (.rotation (Transformation|GetWorldTransform _output_get)))))
  (if (stale EventPickup Distance%20Grab)
    (Physics|Components|PhysicsHandle|GrabComponentatLocationwithRotation _output_get_2 _mesh "None" _returnvalue _returnvalue_2)
    (else
      (Physics|Components|PhysicsHandle|GrabComponentatLocationwithRotation _output_get_2 _mesh "None" (Math|Vector|SelectVector (.Location (Math|Transform|BreakTransform (stale EventPickup Target%20Grab%20Transform))) (.location (Transformation|GetWorldTransform _output_get)) (stale EventPickup Distance%20Grab)) (.rotation (Transformation|GetWorldTransform _output_get)))))
  (CallFunction|StartHandleUpdate))

(event EventForceDrop
  (bind _parent_comp (Variables|Default|GetParent%20Comp))
  (bind _returnvalue (Components|GetOwner _parent_comp))
  ;[1 1 1] Force Drop (Alternate Hand Grabbing)
  (Utilities|IsValid (Variables|Default|GetParent%20Comp)
    (:Is%20Valid
      (Utilities|IsValid _returnvalue
        (:Is%20Valid
          (bind _asbp_motion_controller (Utilities|Casting|CastToBP_MotionController _returnvalue))
          (Default|ReleaseActor _asbp_motion_controller)
          (Rendering|SetVisibility (Variables|Default|GetGrabOffset) false false))))))

(event EventTick
  (params (DeltaSeconds :type Float%20%28single-precision%29))
  ;[1 1 1] TICK
  (CallFunction|TickHandle))

(event EventPickup
  (params (AttachTo :type Scene%20Component%20Object%20Reference) (Distance%20Grab :type Boolean) (Target%20Grab%20Transform :type Transform))
  (bind _grab_snap_type (Variables|Default|GetGrab%20Snap%20Type))
  (bind _graboffset (Variables|Default|GetGrabOffset))
  (bind _returnvalue (Transformation|GetRelativeTransform _graboffset))
  ;[1 1 1] Item Grabbed
  (Input|EnableInput (Game|GetPlayerController 0))
  (switch Utilities|FlowControl|Switch|SwitchonGrabType (Variables|Default|GetGrab%20Type)
    (:NewEnumerator0
      ;[1 1 1] Attachment Grab
      (bind _output_get (Variables|Default|SetParent%20Comp AttachTo))
      (Transformation|AttachComponentToComponent (Variables|Default|GetMesh) _output_get "None" _grab_snap_type _grab_snap_type "KeepWorld" true)
      (if (Variables|Default|GetUse%20Grab%20Offset)
        (Transformation|SetRelativeTransform (Variables|Default|GetMesh) (Math|Transform|InvertTransform (Math|Transform|MakeTransform (.location _returnvalue) (.rotation _returnvalue))) false false)))
    (:NewEnumerator1
      (CallFunction|PhysicsHandleGrab AttachTo Distance%20Grab))
    (:NewEnumerator2
      (CallFunction|ConstraintGrab AttachTo))))

(event EventDrop
  ;[1 1 1] Item Dropped
  (switch Utilities|FlowControl|Switch|SwitchonGrabType (Variables|Default|GetGrab%20Type)
    (:NewEnumerator0
      (Transformation|DetachFromComponent (Variables|Default|GetMesh) "KeepWorld" "KeepWorld" "KeepWorld" true)
      (Physics|SetSimulatePhysics (Variables|Default|GetMesh) true)
      (Variables|Default|SetParent%20Comp 0)
      (Rendering|SetVisibility (Variables|Default|GetGrabOffset) false false))
    (:NewEnumerator1
      (CallFunction|ReleaseHandle))
    (:NewEnumerator2
      (CallFunction|ConstraintRelease))))

(fn ConstructionScript)